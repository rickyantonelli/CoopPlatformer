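; BP_2DPlayer is a 2D player Blueprint with a sprite, a background and a pause menu toggle.
; IA_Pause creates or removes PauseMenu_WB, switching input mode and the MovementEnabled flag, and shows the cursor on opening without hiding it on closing.
; BeginPlay hides Background on non-locally controlled instances.
; The sprite sort priority change sits behind a contradictory nested local-control check, so it never normally runs.
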(event `EnhancedInput|/Game/Dynamic/Blueprints/Input/IA_Pause`
  (params (ActionValue :type Boolean) (ElapsedSeconds :type "Float (double-precision)") (TriggeredSeconds :type "Float (double-precision)") (InputAction :type "InputAction Object Reference" :default "/Game/Dynamic/Blueprints/Input/IA_Pause.IA_Pause"))
  (bind _returnvalue (`GameplayStatics.GetPlayerController` 0))
  ;[1 1 1] Pause Menu
  (:`Triggered`
    (bind _foundwidgets (`WidgetBlueprintLibrary.GetAllWidgetsOfClass` "/Game/Dynamic/Blueprints/UI/WBP/PauseMenu_WB.PauseMenu_WB_C"))
    (if (<= (`KismetArrayLibrary.Array_Length` _foundwidgets) 0)
      (bind _returnvalue_2 (`|CreateWidget` "/Game/Dynamic/Blueprints/UI/WBP/PauseMenu_WB.PauseMenu_WB_C" _returnvalue))
      (`UserWidget.AddToViewport` _returnvalue_2 0)
      (set `PlayerController.bShowMouseCursor` true _returnvalue)
      (`WidgetBlueprintLibrary.SetInputMode_GameAndUIEx` _returnvalue null)
      (set `self.MovementEnabled` false)
      (else
        (`Widget.RemoveFromParent` (`|GetArrayItem` _foundwidgets))
        (`WidgetBlueprintLibrary.SetInputMode_GameOnly` _returnvalue)
        (set `self.MovementEnabled` true)))))

(event `self.ReceiveBeginPlay`
  (bind _returnvalue (`self.IsLocallyControlled`))
  (if (not _returnvalue)
    (`SceneComponent.SetVisibility` (`self.Background`) false false)
    (if _returnvalue
      (`PrimitiveComponent.SetTranslucentSortPriority` (`self.Sprite`) 3))))

(fn `UserConstructionScript`)